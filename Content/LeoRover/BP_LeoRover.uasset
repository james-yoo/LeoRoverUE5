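; Player-driven four-wheel Leo Rover that moves on physics-constraint wheels with skid-style differential steering.
; Forward, turn and brake axes set torque variables, with turning halved at full throttle.
; Tick sums them, mirroring forward drive on the right side, and feeds each wheel constraint's angular velocity target, so the "torques" act as speeds.
; Look axes rotate the camera spring arm.
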(event EventTick
  (params (DeltaSeconds :type Float%20%28single-precision%29))
  ;[1 1 1] Setting up wheel torques
  (Variables|Default|SetWheelFrontLeftTorque (+ (* (Variables|Default|GetForwardTorque) 1.0) (* (Variables|Default|GetWheelFrontLeftTurnTorque) 1.0)))
  (Variables|Default|SetWheelRearLeftTorque (+ (* (Variables|Default|GetForwardTorque) 1.0) (* (Variables|Default|GetWheelRearLeftTurnTorque) 1.0)))
  (Variables|Default|SetWheelFrontRightTorque (+ (* (Variables|Default|GetForwardTorque) -1.0) (* (Variables|Default|GetWheelFrontRightTurnTorque) 1.0)))
  (Variables|Default|SetWheelRearRightTorque (+ (* (Variables|Default|GetForwardTorque) -1.0) (* (Variables|Default|GetWheelRearRightTurnTorque) 1.0)))
  (Class|PhysicsConstraintComponent|SetAngularVelocityTarget (Variables|Default|GetPC_WheelFL) (Math|Vector|MakeVector (Variables|Default|GetWheelFrontLeftTorque) 0.0 0.0))
  (Class|PhysicsConstraintComponent|SetAngularVelocityTarget (Variables|Default|GetPC_WheelRL) (Math|Vector|MakeVector (Variables|Default|GetWheelRearLeftTorque) 0.0 0.0))
  (Class|PhysicsConstraintComponent|SetAngularVelocityTarget (Variables|Default|GetPC_WheelFR) (Math|Vector|MakeVector (Variables|Default|GetWheelFrontRightTorque) 0.0 0.0))
  (Class|PhysicsConstraintComponent|SetAngularVelocityTarget (Variables|Default|GetPC_WheelRR) (Math|Vector|MakeVector (Variables|Default|GetWheelRearRightTorque) 0.0 0.0)))

(event Input|AxisEvents|InputAxisLookUp
  (params (AxisValue :type Float%20%28single-precision%29))
  ;[1 1 1] Camera Control
  (Transformation|AddRelativeRotation (Variables|Default|GetSpringArm) (Math|Rotator|MakeRotator 0.0 AxisValue 0.0) false false))

(event Input|AxisEvents|InputAxisLookRight
  (params (AxisValue :type Float%20%28single-precision%29))
  ;[1 1 1] Camera Control
  (Transformation|AddRelativeRotation (Variables|Default|GetSpringArm) (Math|Rotator|MakeRotator 0.0 0.0 AxisValue) false false))

(event Input|AxisEvents|InputAxisBrake
  (params (AxisValue :type Float%20%28single-precision%29))
  ;[1 1 1] Setting up brake
  (Variables|Default|SetForwardTorque 0.0)
  (Variables|Default|SetWheelFrontLeftTurnTorque 0.0)
  (Variables|Default|SetWheelFrontRightTurnTorque 0.0)
  (Variables|Default|SetWheelRearLeftTurnTorque 0.0)
  (Variables|Default|SetWheelRearRightTurnTorque 0.0))

(event Input|AxisEvents|InputAxisMoveForward
  (params (AxisValue :type Float%20%28single-precision%29))
  ;[1 1 1] Setting up Forward Torque
  (bind _output_get (Variables|Default|SetForwardTorque (* AxisValue 1.0)))
  (Variables|Default|SetIsForwarding (or (Math|Float|NearlyEqual(Float) _output_get 1.0 1e-06) (Math|Float|NearlyEqual(Float) _output_get -1.0 1e-06)))
  (Class|PrimitiveComponent|WakeAllRigidBodies (Variables|Default|GetBody)))

(event Input|AxisEvents|InputAxisMoveRight
  (params (AxisValue :type Float%20%28single-precision%29))
  (bind _isforwarding (Variables|Default|GetIsForwarding))
  ;[1 1 1] Setting up Steering Torques
  (if (Math|Float|NearlyEqual(Float) AxisValue 0.0 1e-06)
    (Variables|Default|SetWheelFrontLeftTurnTorque 0.0)
    (Variables|Default|SetWheelRearLeftTurnTorque 0.0)
    (Variables|Default|SetWheelFrontRightTurnTorque 0.0)
    (Variables|Default|SetWheelRearRightTurnTorque 0.0)
    (elif (< AxisValue 0.0)
      (if _isforwarding
        (Variables|Default|SetWheelFrontLeftTurnTorque -0.5)
        (Variables|Default|SetWheelRearLeftTurnTorque -0.5)
        (Variables|Default|SetWheelFrontRightTurnTorque -0.5)
        (Variables|Default|SetWheelRearRightTurnTorque -0.5)
        (else
          (Variables|Default|SetWheelFrontLeftTurnTorque -1.0)
          (Variables|Default|SetWheelRearLeftTurnTorque -1.0)
          (Variables|Default|SetWheelFrontRightTurnTorque -1.0)
          (Variables|Default|SetWheelRearRightTurnTorque -1.0)))
      (elif _isforwarding
        (Variables|Default|SetWheelFrontLeftTurnTorque 0.5)
        (Variables|Default|SetWheelRearLeftTurnTorque 0.5)
        (Variables|Default|SetWheelFrontRightTurnTorque 0.5)
        (Variables|Default|SetWheelRearRightTurnTorque 0.5)
        (else
          (Variables|Default|SetWheelFrontLeftTurnTorque 1.0)
          (Variables|Default|SetWheelRearLeftTurnTorque 1.0)
          (Variables|Default|SetWheelFrontRightTurnTorque 1.0)
          (Variables|Default|SetWheelRearRightTurnTorque 1.0))))))

(fn ConstructionScript)