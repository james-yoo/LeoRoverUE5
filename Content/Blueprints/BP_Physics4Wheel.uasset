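; Four-wheel physics vehicle driven by angular velocity motors on per-wheel physics constraints, with skid steering.
; Move inputs set fixed forward and opposing turn velocities per side and wake the wheel rigid bodies.
; Every Tick reapplies each side's drive strength and sets its wheels' Y velocity target to forward plus turn.
; SpeedUp inputs step velocity scale variables, but the target calculation does not read them.
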(event EventTick
  (params (DeltaSeconds :type Float%20%28single-precision%29))
  (CallFunction|SetAngularDriveParam)
  (CallFunction|SetVelocity))

(event Input|AxisEvents|InputAxisMoveRight
  (params (AxisValue :type Float%20%28single-precision%29))
  ;[1 1 1] Setup Steering Torque
  (if (Math|Float|NearlyEqual(Float) AxisValue 0.0 1e-06)
    (Variables|Default|SetLeftTurnVelocity 0.0)
    (Variables|Default|SetRightTurnVelocity 0.0)
    (else
      (if (> AxisValue 0.0)
        (Variables|Default|SetLeftTurnVelocity 0.5)
        (Variables|Default|SetRightTurnVelocity -0.5)
        (else
          (Variables|Default|SetLeftTurnVelocity -0.5)
          (Variables|Default|SetRightTurnVelocity 0.5)))
      (CallFunction|WakeRigidBody))))

(event Input|AxisEvents|InputAxisMoveForward
  (params (AxisValue :type Float%20%28single-precision%29))
  ;[1 1 1] Setup Forward Torque
  (if (Math|Float|NearlyEqual(Float) AxisValue 0.0 1e-06)
    (Variables|Default|SetLeftVelocity 0.0)
    (Variables|Default|SetRightVelocity 0.0)
    (else
      (if (> AxisValue 0.0)
        (Variables|Default|SetLeftVelocity 1.0)
        (Variables|Default|SetRightVelocity 1.0)
        (else
          (Variables|Default|SetLeftVelocity -1.0)
          (Variables|Default|SetRightVelocity -1.0)))
      (CallFunction|WakeRigidBody))))

(event Input|AxisEvents|InputAxisForwardSpeedUp
  (params (AxisValue :type Float%20%28single-precision%29))
  ;[1 1 1] Configure Forward SpeedUp
  (if (not (Math|Float|NearlyEqual(Float) AxisValue 0.0 1e-06))
    (if (> AxisValue 0.0)
      (Variables|Default|SetLeftVelocityScale (+ (Variables|Default|GetLeftVelocityScale) 0.1))
      (Variables|Default|SetRightVelocityScale (+ (Variables|Default|GetRightVelocityScale) 0.1))
      (else
        (Variables|Default|SetLeftVelocityScale (- (Variables|Default|GetLeftVelocityScale) 0.1))
        (Variables|Default|SetRightVelocityScale (- (Variables|Default|GetRightVelocityScale) 0.1))))))

(event Input|AxisEvents|InputAxisTurnSpeedUp
  (params (AxisValue :type Float%20%28single-precision%29))
  ;[1 1 1] Configure Turn SpeedUp
  (if (not (Math|Float|NearlyEqual(Float) AxisValue 0.0 1e-06))
    (if (> AxisValue 0.0)
      (Variables|Default|SetLeftTurnVelocityScale (+ (Variables|Default|GetLeftTurnVelocityScale) 0.1))
      (Variables|Default|SetRightTurnVelocityScale (- (Variables|Default|GetRightTurnVelocityScale) 0.1))
      (else
        (Variables|Default|SetLeftTurnVelocityScale (- (Variables|Default|GetLeftTurnVelocityScale) 0.1))
        (Variables|Default|SetRightTurnVelocityScale (+ (Variables|Default|GetRightTurnVelocityScale) 0.1))))))

(fn ConstructionScript)

(fn WakeRigidBody
  (Class|PrimitiveComponent|WakeAllRigidBodies (Variables|Default|GetWheelFL))
  (Class|PrimitiveComponent|WakeAllRigidBodies (Variables|Default|GetWheelRL))
  (Class|PrimitiveComponent|WakeAllRigidBodies (Variables|Default|GetWheelFR))
  (Class|PrimitiveComponent|WakeAllRigidBodies (Variables|Default|GetWheelRR)))

(fn SetVelocity
  (bind _leftturnvelocity (Variables|Default|GetLeftTurnVelocity))
  (bind _leftvelocity (Variables|Default|GetLeftVelocity))
  (bind _rightvelocity (Variables|Default|GetRightVelocity))
  (bind _rightturnvelocity (Variables|Default|GetRightTurnVelocity))
  (bind _returnvalue (+ _leftvelocity _leftturnvelocity))
  (bind _returnvalue_2 (+ _rightvelocity _rightturnvelocity))
  (Class|PhysicsConstraintComponent|SetAngularVelocityTarget (Variables|Default|GetPC_BaseFL) (Math|Vector|MakeVector 0.0 _returnvalue 0.0))
  (Class|PhysicsConstraintComponent|SetAngularVelocityTarget (Variables|Default|GetPC_BaseRL) (Math|Vector|MakeVector 0.0 _returnvalue 0.0))
  (Class|PhysicsConstraintComponent|SetAngularVelocityTarget (Variables|Default|GetPC_BaseFR) (Math|Vector|MakeVector 0.0 _returnvalue_2 0.0))
  (Class|PhysicsConstraintComponent|SetAngularVelocityTarget (Variables|Default|GetPC_BaseRR) (Math|Vector|MakeVector 0.0 _returnvalue_2 0.0)))

(fn SetAngularDriveParam
  (bind _leftvelocitystrength (Variables|Default|GetLeftVelocityStrength))
  (bind _rightvelocitystrength (Variables|Default|GetRightVelocityStrength))
  (Class|PhysicsConstraintComponent|SetAngularDriveParams (Variables|Default|GetPC_BaseFL) 0.0 _leftvelocitystrength 0.0)
  (Class|PhysicsConstraintComponent|SetAngularDriveParams (Variables|Default|GetPC_BaseRL) 0.0 _leftvelocitystrength 0.0)
  (Class|PhysicsConstraintComponent|SetAngularDriveParams (Variables|Default|GetPC_BaseFR) 0.0 _rightvelocitystrength 0.0)
  (Class|PhysicsConstraintComponent|SetAngularDriveParams (Variables|Default|GetPC_BaseRR) 0.0 _rightvelocitystrength 0.0))