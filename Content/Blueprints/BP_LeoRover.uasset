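; Player-controlled Leo Rover that drives with four physics-constraint wheels and skid steering, with a spring-arm camera rotated by look input.
; Move axes set forward and fixed-magnitude turn values, which Tick mixes into left and right wheel speeds, mirroring the forward sign.
; Despite their "Torque" names, these values feed the constraints' angular velocity targets and are printed each frame for debugging.
; Pressing Brake zeroes all drive values once.
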(event EventBeginPlay)

(event Collision|EventActorBeginOverlap
  (params (OtherActor :type Actor%20Object%20Reference)))

(event EventTick
  (params (DeltaSeconds :type Float%20%28single-precision%29))
  (Variables|Default|SetWheelLeftTorque (+ (* (Variables|Default|GetForwardTorque) -1.0) (* (Variables|Default|GetWheelLeftTurnTorque) 2.0)))
  (Variables|Default|SetWheelRightTorque (+ (* (Variables|Default|GetForwardTorque) 1.0) (* (Variables|Default|GetWheelRightTurnTorque) 2.0)))
  (Class|PhysicsConstraintComponent|SetAngularVelocityTarget (Variables|Default|GetPC_WheelFL) (Math|Vector|MakeVector 0.0 (Variables|Default|GetWheelLeftTorque) 0.0))
  (Class|PhysicsConstraintComponent|SetAngularVelocityTarget (Variables|Default|GetPC_WheelRL) (Math|Vector|MakeVector 0.0 (Variables|Default|GetWheelLeftTorque) 0.0))
  (Class|PhysicsConstraintComponent|SetAngularVelocityTarget (Variables|Default|GetPC_WheelFR) (Math|Vector|MakeVector 0.0 (Variables|Default|GetWheelRightTorque) 0.0))
  (Class|PhysicsConstraintComponent|SetAngularVelocityTarget (Variables|Default|GetPC_WheelRR) (Math|Vector|MakeVector 0.0 (Variables|Default|GetWheelRightTorque) 0.0))
  (Development|PrintText (Utilities|Text|ToText(String) (Utilities|String|Append (Utilities|String|ToString(Float) (Variables|Default|GetWheelLeftTorque)) ", " (Utilities|String|ToString(Float) (Variables|Default|GetWheelRightTorque))))))

(event Input|ActionEvents|InputActionBrake
  (params (Key :type Key%20Structure :default "None"))
  ;[1 1 1] Setting up Brake
  (:Pressed
    (Variables|Default|SetForwardTorque 0.0)
    (Variables|Default|SetWheelLeftTorque 0.0)
    (Variables|Default|SetWheelRightTorque 0.0)
    (Variables|Default|SetWheelLeftTurnTorque 0.0)
    (Variables|Default|SetWheelRightTurnTorque 0.0)))

(event Input|AxisEvents|InputAxisLookUp
  (params (AxisValue :type Float%20%28single-precision%29))
  ;[1 1 1] Camera Control
  (Transformation|AddRelativeRotation (Variables|Default|GetSpringArm) (Math|Rotator|MakeRotator 0.0 AxisValue 0.0) false false))

(event Input|AxisEvents|InputAxisLookRight
  (params (AxisValue :type Float%20%28single-precision%29))
  ;[1 1 1] Camera Control
  (Transformation|AddRelativeRotation (Variables|Default|GetSpringArm) (Math|Rotator|MakeRotator 0.0 0.0 AxisValue) false false))

(event Input|AxisEvents|InputAxisMoveForward
  (params (AxisValue :type Float%20%28single-precision%29))
  ;[1 1 1] Setting up Forward Torque
  (Variables|Default|SetForwardTorque (* AxisValue 5.0)))

(event Input|AxisEvents|InputAxisMoveRight
  (params (AxisValue :type Float%20%28single-precision%29))
  ;[1 1 1] Setting up Steering Torques
  (if (Math|Float|NearlyEqual(Float) AxisValue 0.0 1e-06)
    (Variables|Default|SetWheelLeftTurnTorque 0.0)
    (Variables|Default|SetWheelRightTurnTorque 0.0)
    (elif (< AxisValue 0.0)
      (Variables|Default|SetWheelLeftTurnTorque 1.0)
      (Variables|Default|SetWheelRightTurnTorque 1.0)
      (else
        (Variables|Default|SetWheelLeftTurnTorque -1.0)
        (Variables|Default|SetWheelRightTurnTorque -1.0)))))

(fn ConstructionScript)